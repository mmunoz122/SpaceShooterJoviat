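; BP_EnemyBase is the base enemy for a space shooter, flying in a straight line and firing at regular intervals.
; BeginPlay stores the forward vector, and Tick moves the actor along it by Speed without sweep while accumulating a shot timer.
; When the timer passes DelayShoot, Fire spawns the EnemyBullet class at the FirePoint transform and the timer resets.
; Two custom events duplicate the BeginPlay and Tick logic.
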(event Custom|CustomEvent
  ;[0.15 0.15 0.15 0.5] Event - EnemyBase
  (Variables|Default|SetMovementVector (Transformation|GetActorForwardVector)))

(event Custom|CustomEvent_1
  (params (DeltaSeconds :type Float%20%28single-precision%29))
  ;[0.15 0.15 0.15 0.5] Event - EnemyBase
  (Transformation|SetActorLocation (+ (Transformation|GetActorLocation) (* (* DeltaSeconds (Variables|Default|GetSpeed)) (Variables|Default|GetMovementVector))) false false)
  (Variables|Default|SetShootCurrentTime (+ (Variables|Default|GetShootCurrentTime) DeltaSeconds))
  (if (> (Variables|Default|GetShootCurrentTime) (Variables|Default|GetDelayShoot))
    (CallFunction|Fire)
    (Variables|Default|SetShootCurrentTime 0.0)))

(event EventBeginPlay
  ;[0.15 0.15 0.15 0.5] Event - BeginPlay
  (Variables|Default|SetMovementVector (Transformation|GetActorForwardVector)))

(event EventTick
  (params (DeltaSeconds :type Float%20%28single-precision%29))
  ;[0.15 0.15 0.15 0.5] Function - GetClassToSpawn
  (Transformation|SetActorLocation (+ (Transformation|GetActorLocation) (* (* DeltaSeconds (Variables|Default|GetSpeed)) (Variables|Default|GetMovementVector))) false false)
  (Variables|Default|SetShootCurrentTime (+ (Variables|Default|GetShootCurrentTime) DeltaSeconds))
  (if (> (Variables|Default|GetShootCurrentTime) (Variables|Default|GetDelayShoot))
    (CallFunction|Fire)
    (Variables|Default|SetShootCurrentTime 0.0)))

(fn ConstructionScript)

(fn Fire
  (Game|SpawnActorfromClass "/Game/00_Space_Shooter/Enemies/EnemyBullet.EnemyBullet_C" (Transformation|GetWorldTransform (Variables|Default|GetFirePoint)) "Undefined" "MultiplyWithRoot" 0 0))