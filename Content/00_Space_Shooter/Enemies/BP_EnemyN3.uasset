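; BP_EnemyN3 is a space shooter enemy that moves toward the player and fires.
; Each tick it issues AIMoveTo on the player character and also shifts itself along the forward vector cached at BeginPlay, repeating that step on move success.
; The shot timer multiplies by delta time instead of adding, and both branches of the delay check call Fire, so it fires every time that step runs.
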(event Custom|Event%20Tick
  (params (DeltaSeconds :type Float%20%28single-precision%29))
  ;[1 1 1] Comment
  (AI|AIMoveTo (Variables|Default|GetPawn) "0, 0, 0" (Game|GetPlayerCharacter 0) 1e+02 false
    (:then
      _)
    (:OnSuccess
      _))
  (Transformation|SetActorLocation (+ (Transformation|GetActorLocation) (* (* DeltaSeconds (Variables|Default|GetSpeed)) (Variables|Default|GetMovementVector))) false false)
  (Variables|Default|SetShootCurrentTime (* (Variables|Default|GetShootCurrentTime) DeltaSeconds))
  (if (> (Variables|Default|GetShootCurrentTime) (Variables|Default|GetDelayShoot))
    (CallFunction|Fire)
    (Variables|Default|SetShootCurrentTime 0.0)
    (else
      (CallFunction|Fire))))

(event EventBeginPlay
  ;[1 1 1] Comment
  (Variables|Default|SetMovementVector (Transformation|GetActorForwardVector)))

(fn ConstructionScript
  (|CallParentFunction))