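; BP_EnemyN1 is a space shooter enemy that spins while flying in a straight line and firing at intervals.
; It caches its forward vector on BeginPlay and moves along it each tick at Speed scaled by delta time, without sweep, so its spin does not bend the path.
; The local yaw spin is a fixed step per frame, and a tick-accumulated timer calls Fire whenever DelayShoot is exceeded.
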(event EventBeginPlay
  ;[0.15 0.15 0.15 0.5] Event - BeginPlay
  (Variables|Default|SetMovementVector (Transformation|GetActorForwardVector)))

(event EventTick
  (params (DeltaSeconds :type Float%20%28single-precision%29))
  ;[0.15 0.15 0.15 0.5] Event - Event Tick
  (Transformation|AddActorLocalRotation "0.000000,30.000000,0.000000" false false)
  (Transformation|SetActorLocation (+ (Transformation|GetActorLocation) (* (* DeltaSeconds (Variables|Default|GetSpeed)) (Variables|Default|GetMovementVector))) false false)
  (Variables|Default|SetShootCurrentTime (+ (Variables|Default|GetShootCurrentTime) DeltaSeconds))
  (if (> (Variables|Default|GetShootCurrentTime) (Variables|Default|GetDelayShoot))
    (CallFunction|Fire)
    (Variables|Default|SetShootCurrentTime 0.0)))

(fn ConstructionScript
  (|CallParentFunction))