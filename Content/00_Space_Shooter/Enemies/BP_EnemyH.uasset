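; BP_EnemyH is a space shooter enemy variant that moves along its right vector, judging by the MovementVector it sets on BeginPlay.
; It reverses that vector whenever it overlaps an actor tagged "Lateral", giving a side-to-side bounce between such actors.
; It only sets the direction; applying the movement is left outside this Blueprint, presumably to its parent class, and its own Tick is disabled.
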(event EventBeginPlay
  ;[0.15 0.15 0.15 0.5] Event - BeginPlay
  (|CallParentFunction)
  (Variables|Default|SetMovementVector (Transformation|GetActorRightVector)))

(event Collision|EventActorBeginOverlap
  (params (OtherActor :type Actor%20Object%20Reference))
  ;[0.15 0.15 0.15 0.5] Event - ActorBeginOverlap
  (|CallParentFunction OtherActor)
  (if (Utilities|Array|ContainsItem (Variables|/Script/Engine.Actor|GetTags OtherActor) "Lateral")
    (Variables|Default|SetMovementVector (* (Variables|Default|GetMovementVector) "-1.000000,-1.000000,-1.000000"))))

(event EventTick
  (params (DeltaSeconds :type Float%20%28single-precision%29))
  (|CallParentFunction DeltaSeconds) ; This node is disabled and will not be called.\nDrag off pins to build functionality.
)

(fn ConstructionScript
  (|CallParentFunction))